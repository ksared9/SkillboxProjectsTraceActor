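; BP_CubeMoveComp is an actor that cycles MovingComp between two target cubes and its starting position.
; BeginPlay caches the component's relative location, then chains timed MoveComponentTo moves to TargetCube and TargetCube1, each followed by a matching Delay.
; A quicker move returns it to the cached location, and after a short Delay execution wires back into a single-iteration loop, repeating the cycle endlessly without Tick.
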(event EventBeginPlay
  (Variables|Default|SetRelative%20Location (Variables|/Script/Engine.SceneComponent|GetRelativeLocation (Variables|Default|GetMovingComp)))
  (for _index (range 0 0) :!label _label
    (Components|MoveComponentTo (Variables|Default|GetMovingComp) (Variables|/Script/Engine.SceneComponent|GetRelativeLocation (Variables|Default|GetTargetCube)) "0, 0, 0" false false 4.0 false)
    (Utilities|FlowControl|Delay 4.0)
    (Components|MoveComponentTo (Variables|Default|GetMovingComp) (Variables|/Script/Engine.SceneComponent|GetRelativeLocation (Variables|Default|GetTargetCube1)) "0, 0, 0" false false 3.0 false)
    (Utilities|FlowControl|Delay 3.0)
    (Components|MoveComponentTo (Variables|Default|GetMovingComp) (Variables|Default|GetRelative%20Location) "0, 0, 0" false false 0.2 false)
    (Utilities|FlowControl|Delay 0.5)
    (goto _label)))

(event Collision|EventActorBeginOverlap
  (params (OtherActor :type Actor%20Object%20Reference)))

(event EventTick
  (params (DeltaSeconds :type Float%20%28single-precision%29)))

(fn ConstructionScript)